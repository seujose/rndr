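; Player character that serves as the viewport camera and selection controller for a V-Ray rendering scene editor.
; Alt plus mouse buttons orbit, pan and zoom the spring-arm camera, alongside movement axes and fit-to-selection.
; Clicks multi-trace for RndrBaseActor meshes or axis handles that open move gates.
; VrayInterfaceBP receives selection, deletion and camera updates; other keys toggle MasterWidget, feed it pixel data and adjust post-process exposure.
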(event `self.ReceiveTick`
  (params (DeltaSeconds :type "Float (single-precision)"))
  (`SceneComponent.K2_SetWorldRotation` (`self.Arrow1`) (struct :`Roll` 90.0) false false)
  (`SceneComponent.K2_SetWorldRotation` (`self.Arrow2`) (struct :`Yaw` 90.0) false false)
  (`SceneComponent.K2_SetWorldRotation` (`self.Arrow3`) (struct :`Pitch` 90.0 :`Yaw` 90.0) false false))

(event `self.ReceiveBeginPlay`
  (bind _outactors (`GameplayStatics.GetAllActorsOfClass` "/Script/Engine.PostProcessVolume"))
  (set `self.postProcess` (`|GetArrayItem` _outactors))
  (bind _returnvalue (`|CreateWidget` "/Game/MasterWidget.MasterWidget_C"))
  (bind _output_get (set `self.masterWidget` _returnvalue))
  (`UserWidget.AddToViewport` _output_get 0))

(event `Key|Down`
  (params (Key :type "Key Structure"))
  (:`Pressed`
    (set `self.exposure` -1.0)
    (set `PostProcessVolume.Settings` (make `PostProcessSettings` :`AutoExposureBias` (+ (`.AutoExposureBias` (break `PostProcessSettings` (`PostProcessVolume.Settings` (`self.postProcess`)))) (`self.exposure`))) (`self.postProcess`) :!label _label)))

(event `Key|Up`
  (params (Key :type "Key Structure"))
  (:`Pressed`
    (set `self.exposure` 1.0)
    (goto _label)))

(event `Key|LeftMouseButton`
  (params (Key :type "Key Structure"))
  (:`Pressed`
    (if (not (`PlayerController.IsInputKeyDown` (`GameplayStatics.GetPlayerController` 0) "LeftAlt"))
      (`self.setSelection`))))

(event `Key|Delete`
  (params (Key :type "Key Structure"))
  (:`Pressed`
    (`/Game/VrayInterfaceBP.Delete` (`self.getVray`))))

(event `Key|Escape`
  (params (Key :type "Key Structure"))
  (:`Pressed`
    (bind _foundwidgets (`WidgetBlueprintLibrary.GetAllWidgetsOfClass` "/Game/MasterWidget.MasterWidget_C" false))
    (for _array_element _foundwidgets
      (bind _properties (`/Game/MasterWidget.Properties` _array_element))
      (if (`Widget.IsVisible` _properties)
        (`Widget.SetVisibility` _properties "Collapsed")
        (else
          (`Widget.SetVisibility` _properties "Visible"))))))

(event `Key|F`
  (params (Key :type "Key Structure"))
  (bind _output (`|GetArrayItem` (`/Game/VrayInterfaceBP.GetSelection` (`self.getVray`))))
  (:`Pressed`
    (`/Engine/EditorBlueprintResources/StandardMacros.IsValid` _output
      (:`Is Valid`
        (`self.K2_SetActorLocation` (cast `/Game/RndrCharacterBP` (`GameplayStatics.GetPlayerCharacter` 0) :!pure true) (`self.K2_GetActorLocation` _output) false true)
        (`SceneComponent.K2_SetRelativeLocation` (`self.SpringArm`) (0.0 0.0 0.0) false false)
        (set `SpringArmComponent.TargetArmLength` 80.0 (`self.SpringArm`))))))

(event `Key|LeftControl`
  (params (Key :type "Key Structure"))
  (:`Pressed`
    (`VrayInterface.updateView` (`self.getVray`) (`self.getView`))))

(event `Key|T`
  (params (Key :type "Key Structure"))
  (:`Pressed`
    (bind _outtexture (`VrayInterface.getPixelDataaa` (`self.getVray`)))
    (set `/Game/MasterWidget.destinaTex` _outtexture (`self.masterWidget`))))

(event `InputAxisKey|MouseWheelAxis`
  (params (AxisValue :type "Float (single-precision)"))
  ;[1 1 1] zoom
  (set `SpringArmComponent.TargetArmLength` (+ (`SpringArmComponent.TargetArmLength` (`self.SpringArm`)) (* AxisValue -100.0)) (`self.SpringArm`)))

(event `InputAxis|orbit`
  (params (AxisValue :type "Float (single-precision)"))
  ;[1 1 1] orbit
  (if (and (`PlayerController.IsInputKeyDown` (`GameplayStatics.GetPlayerController` 0) "LeftAlt") (`PlayerController.IsInputKeyDown` (`GameplayStatics.GetPlayerController` 0) "LeftMouseButton"))
    (`self.AddControllerYawInput` (* 2 (`self.GetInputAxisKeyValue`)))
    (`self.AddControllerPitchInput` (* -2 (`self.GetInputAxisKeyValue`)))))

(event `InputAxis|panner`
  (params (AxisValue :type "Float (single-precision)"))
  ;[1 1 1] pan
  (if (and (`PlayerController.IsInputKeyDown` (`GameplayStatics.GetPlayerController` 0) "LeftAlt") (`PlayerController.IsInputKeyDown` (`GameplayStatics.GetPlayerController` 0) "MiddleMouseButton"))
    (`SceneComponent.K2_AddLocalOffset` (`self.SpringArm`) (`KismetMathLibrary.MakeVector` 0.0 (* (`self.GetInputAxisKeyValue`) (`self.panMultiplier`)) (* (`self.GetInputAxisKeyValue`) (`self.panMultiplier`))) false false)))

(event `InputAxis|zoom`
  (params (AxisValue :type "Float (single-precision)"))
  ;[1 1 1] zoom
  (if (and (`PlayerController.IsInputKeyDown` (`GameplayStatics.GetPlayerController` 0) "LeftAlt") (`PlayerController.IsInputKeyDown` (`GameplayStatics.GetPlayerController` 0) "RightMouseButton"))
    (set `SpringArmComponent.TargetArmLength` (+ (`SpringArmComponent.TargetArmLength` (`self.SpringArm`)) (* (`self.GetInputAxisKeyValue`) -10.0)) (`self.SpringArm`))))

(event `InputAxis|moveForward`
  (params (AxisValue :type "Float (single-precision)"))
  (`self.AddMovementInput` (`KismetMathLibrary.GetForwardVector` (`KismetMathLibrary.MakeRotator` 0.0 0.0 (.yaw (`self.GetControlRotation`)))) AxisValue))

(event `InputAxis|moveRight`
  (params (AxisValue :type "Float (single-precision)"))
  (`self.AddMovementInput` (`KismetMathLibrary.GetRightVector` (`KismetMathLibrary.MakeRotator` 0.0 0.0 (.yaw (`self.GetControlRotation`)))) AxisValue))

(event `InputAxis|MoveUp`
  (params (AxisValue :type "Float (single-precision)"))
  (`self.AddMovementInput` (`KismetMathLibrary.GetUpVector` (`KismetMathLibrary.MakeRotator` 0.0 0.0 (.yaw (`self.GetControlRotation`)))) AxisValue))

(fn `getfaceUnderMouse`
  (locals (HitResult :type "Vector Structure" :default (0.0 0.0 0.0)) (hitNormal :type "Vector Structure" :default (0.0 0.0 0.0)))
  (bind _hitresult (`PlayerController.GetHitResultUnderCursorByChannel` (`GameplayStatics.GetPlayerController` 0) "TraceTypeQuery1" true))
  (set `local.HitResult` (`.Location` (`GameplayStatics.BreakHitResult` _hitresult)))
  (set `self.HitNormall` (`.Normal` (`GameplayStatics.BreakHitResult` _hitresult)))
  (bind _hitout (`self.MaTrace` self (+ (`local.HitResult`) (* (`self.HitNormall`) 10)) (- (`local.HitResult`) (* (`self.HitNormall`) 10)) "ECC_Visibility"))
  (if (!= (`.FaceIndex` (`GameplayStatics.BreakHitResult` _hitout)) -1)
    (set `self.faceunderMouse` (`.FaceIndex` (`GameplayStatics.BreakHitResult` _hitout)))
    (`KismetSystemLibrary.DrawDebugLine` (+ (`local.HitResult`) (* (`self.HitNormall`) 10)) (- (`local.HitResult`) (* (`self.HitNormall`) 10)) (struct :`R` 1.0 :`G` 1.0 :`B` 1.0 :`A` 1.0) 2.0 1.0)
    (return)
    (else
      (return))))

(fn `getView`
  (returns (Array :type "Array of Vector Structure"))
  (bind _camera (`self.Camera`))
  (return (`|MakeArray` (`SceneComponent.GetRightVector` _camera) (`SceneComponent.GetUpVector` _camera) (* (`SceneComponent.GetForwardVector` _camera) -1) (`SceneComponent.K2_GetComponentLocation` (`self.Camera`)))))

(fn `getVray`
  (returns (VrayInterface :type "/Game/VrayInterfaceBP Object Reference"))
  (bind _outactors (`GameplayStatics.GetAllActorsOfClass` "/Game/VrayInterfaceBP.VrayInterfaceBP_C"))
  (return (`|GetArrayItem` _outactors)))

(fn `setSelection`
  (locals (baseActorArrowComponents :type "Array of PrimitiveComponent Object Reference") (outHit :type "Array of HitResult Structure") (selectedActor :type "/Game/RndrBaseActor Object Reference") (axis :type Integer :default 0) (hitCompo :type "PrimitiveComponent Object Reference"))
  (bind (_worldlocation _worlddirection) (`PlayerController.DeprojectMousePositionToWorld` (`GameplayStatics.GetPlayerController` 0)))
  (bind (_bblockinghit _binitialoverlap _time _distance _location _impactpoint _normal _impactnormal _physmat _hitactor _hitcomponent) (`GameplayStatics.BreakHitResult` (`|GetArrayItem` (`local.outHit`))))
  (bind _outhits (`KismetSystemLibrary.LineTraceMulti` :`Start` _worldlocation :`End` (+ _worldlocation (* _worlddirection 100000)) :`TraceChannel` "TraceTypeQuery1" :`bTraceComplex` true :`DrawDebugType` "ForDuration"))
  (set `local.outHit` _outhits)
  (if (`KismetArrayLibrary.Array_IsValidIndex` (`local.outHit`))
    (if (`KismetArrayLibrary.Array_IsValidIndex` (`/Game/VrayInterfaceBP.GetSelection` (`self.getVray`)))
      (set `local.selectedActor` (`|GetArrayItem` (`/Game/VrayInterfaceBP.GetSelection` (`self.getVray`))))
      (for _array_element (`local.outHit`)
        (set `local.hitCompo` (`.HitComponent` (`GameplayStatics.BreakHitResult` _array_element)))
        (if (`ActorComponent.ComponentHasTag` (`local.hitCompo`) "axis")
          (if (== (`ActorComponent.GetOwner` (`local.hitCompo`)) (`local.selectedActor`))
            (switch `string` (`KismetSystemLibrary.GetObjectName` (`local.hitCompo`))
              (:`x_axis`
                (set `local.axis` 0))
              (:`y_axis`
                (set `local.axis` 1))
              (:`z_axis`
                (set `local.axis` 2)))
            (`/Game/RndrBaseActor.openMoveGate` (`local.selectedActor`) (`local.axis`))
            (break))))
      (bind _asrndr_base_actor (cast `/Game/RndrBaseActor` (`ActorComponent.GetOwner` (`local.hitCompo`))))
      (`/Game/VrayInterfaceBP.SetSelectionRndrd` (`self.getVray`) _asrndr_base_actor)
      (elif (`ActorComponent.ComponentHasTag` _hitcomponent "visualMesh")
        (bind _asrndr_base_actor_2 (cast `/Game/RndrBaseActor` _hitactor))
        (`/Game/VrayInterfaceBP.SetSelectionRndrd` (`self.getVray`) _asrndr_base_actor_2)))
    (else
      (`/Game/VrayInterfaceBP.SetSelectionRndrd` (`self.getVray`) null)
      (return))))

(fn `UserConstructionScript`)