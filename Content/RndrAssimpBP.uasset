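; Runtime model importer that spawns scene nodes from a file and mirrors them into V-Ray.
; BeginPlay caches the master UI and V-Ray interface actor.
; FnSpawnNode spawns a procedural-mesh RndrBaseActor_Node per mesh entry, negating Y/Z position and pitch/yaw.
; It re-reads the file with LeftHanded off for each V-Ray static mesh, sets diffuse color/texture and transform, syncs the material and refreshes the scene browser.
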(event `self.ReceiveBeginPlay`
  (`KismetSystemLibrary.Delay` 0.2)
  (bind _foundwidgets (`VictoryBPFunctionLibrary.GetAllWidgetsOfClass` "/Game/MasterWidget.MasterWidget_C"))
  (set `self.masterUI` (`|GetArrayItem` _foundwidgets))
  (bind _outactors (`GameplayStatics.GetAllActorsOfClass` "/Game/VrayInterfaceBP.VrayInterfaceBP_C"))
  (bind _output (`|GetArrayItem` _outactors))
  (`/Engine/EditorBlueprintResources/StandardMacros.IsValid` _output
    (:`Is Valid`
      (set `self.vray` _output))
    (:`Is Not Valid`
      (`/Game/MasterWidget.setUserMessage` (`self.masterUI`) "interface vray invalida" (make `SlateColor` (struct :`R` 1.0 :`A` 1.0))))))

(fn `fn_spawnNode`
  (params (FilePath :type String))
  (locals (theNode :type "/Game/RndrBaseActor_Node Object Reference") (theFilePath :type String) (thePluginName :type String) (texturesArray :type "Array of String") (matColor :type "LinearColor Structure" :default (struct :`R` 1.0 :`G` 1.0 :`B` 1.0 :`A` 1.0)) (texturePath :type String) (rotation :type "Quat Structure") (positionOut :type "Vector Structure" :default (0.0 0.0 0.0)) (scaleOut :type "Vector Structure" :default (0.0 0.0 0.0)) (unrealVertices :type "Array of Vector Structure") (unrealNormals :type "Array of Vector Structure") (unrealfaces :type "Array of Integer") (unrealuv0 :type "Array of Vector2D Structure") (unrealuv1 :type "Array of Vector2D Structure") (parentPos :type "Vector Structure") (parentRotation :type "Quat Structure") (parentScale :type "Vector Structure") (parentName :type String) (name :type String))
  (bind _thenode (`local.theNode`))
  (bind (_positionout_x _positionout_y _positionout_z) (`KismetMathLibrary.BreakVector` (`local.positionOut`)))
  (bind (_returnvalue_roll _returnvalue_pitch _returnvalue_yaw) (`KismetMathLibrary.BreakRotator` (`KismetMathLibrary.Quat_Rotator` (`local.rotation`))))
  ;[1 1 1] unreal
  (set `local.theFilePath` FilePath)
  (bind (_meshinfoout _returnvalue) (`self.newMeshInfo` (`local.theFilePath`) true))
  (if _returnvalue
    (for (_array_element _array_index) _meshinfoout
      (set `local.texturesArray` (break `MeshInfo` _array_element))
      (set `local.matColor` (`.color` (break `MeshInfo` _array_element)))
      (set `local.positionOut` (`.position` (break `MeshInfo` _array_element)))
      (set `local.rotation` (`.rotation` (break `MeshInfo` _array_element)))
      (set `local.scaleOut` (`.scale` (break `MeshInfo` _array_element)))
      (set `local.name` (`.name` (break `MeshInfo` _array_element)))
      (set `local.parentName` (`.parentName` (break `MeshInfo` _array_element)))
      (set `local.parentPos` (`.parentPosition` (break `MeshInfo` _array_element)))
      (set `local.parentRotation` (`.parentRotation` (break `MeshInfo` _array_element)))
      (set `local.parentScale` (`.parentScale` (break `MeshInfo` _array_element)))
      (`KismetSystemLibrary.PrintString` (`KismetStringLibrary.Concat_StrStr` (`local.name`) "(" (`KismetStringLibrary.Conv_RotatorToString` (`KismetMathLibrary.Quat_Rotator` (`local.rotation`))) ")" (`local.parentName`) "(" (`KismetStringLibrary.Conv_RotatorToString` (`KismetMathLibrary.Quat_Rotator` (`local.parentRotation`))) ")"))
      (bind _returnvalue_2 (`|SpawnActorFromClass` "/Game/RndrBaseActor_Node.RndrBaseActor_Node_C" (`KismetMathLibrary.MakeTransform` (0.0 0.0 0.0)) "AdjustIfPossibleButAlwaysSpawn" "OverrideRootScale" null "" null))
      (bind _output_get (set `local.theNode` _returnvalue_2))
      (`/Game/RndrBaseActor_Node.CreateProceduralMesh` _output_get (`.vertices` (break `MeshInfo` _array_element)) (`.faces` (break `MeshInfo` _array_element)) (`.normals` (break `MeshInfo` _array_element)) (`.uv0` (break `MeshInfo` _array_element)) (`.uv1` (break `MeshInfo` _array_element)))
      (`self.K2_SetActorTransform` (`local.theNode`) (`KismetMathLibrary.MakeTransform` (`KismetMathLibrary.MakeVector` _positionout_x (* -1 _positionout_y) (* -1 _positionout_z)) (`KismetMathLibrary.MakeRotator` _returnvalue_roll (* -1 _returnvalue_pitch) (* -1 _returnvalue_yaw)) (`local.scaleOut`)) false true) ; verificar se exportacao do fbx está em Z como UP axis
      (bind _meshinfoout_2 (`self.newMeshInfo` (`local.theFilePath`)))
      (bind _pluginnameout (`VrayInterface.CreatePluginCpp` (`self.vray`) "ENode" false))
      ;[1 1 1] vray
      (bind _output_get_2 (set `local.thePluginName` _pluginnameout))
      (set `/Game/RndrBaseActor.name` _output_get_2 (`local.theNode`))
      (bind (_output_texturespath _output_color _output_position _output_rotation _output_scale _output_name _output_parentname _output_parentposition _output_parentrotation _output_parentscale _output_vertices _output_normals _output_faces _output_facenormals _output_uv0 _output_uv1) (break `MeshInfo` (`|GetArrayItem` _meshinfoout_2 _array_index)))
      (`VrayInterface.CreateGeomStaticMesh` (`self.vray`) _output_uv0 _output_uv1 _output_vertices _output_normals _output_faces _output_faces (`local.thePluginName`))
      ;;[1 0 0] Comment
      (if (`KismetArrayLibrary.Array_IsValidIndex` (`local.texturesArray`))
        (set `local.texturePath` (`KismetStringLibrary.Replace` (`|GetArrayItem` (`local.texturesArray`)) "..\\..\\..\\..\\.." "C:"))
        (else
          (set `local.texturePath` "")))
      (`VrayInterface.SetVrayPluginParameter` :`self` (`self.vray`) :`PluginType` "EBRDF" :`nameIn` (`local.thePluginName`) :`colorIn` (`local.matColor`) :`ParameterName` "diffuse" :`stringIn` (`local.texturePath`))
      (`VrayInterface.SetVrayPluginParameter` :`self` (`self.vray`) :`PluginType` "ENode" :`transformIn` (`|MakeArray` (`self.GetActorForwardVector` _thenode) (`self.GetActorRightVector` _thenode) (`self.GetActorUpVector` _thenode) (`self.K2_GetActorLocation` (`local.theNode`))) :`nameIn` (`local.thePluginName`) :`ParameterName` "transform")
      (`/Game/RndrBaseActor_Node.syncMat` (`local.theNode`))
      (`/Game/MasterWidget.RefreshSceneBrowser` (`self.masterUI`)))))

(fn `NewFunction_0`
  (params (parent :type "Quat Structure (by ref)") (Q1 :type "Quat Structure (by ref)") (`T Location` :type "Vector Structure"))
  (returns (ReturnValue :type "Rotator Structure"))
  (bind (_returnvalue_roll _returnvalue_pitch _returnvalue_yaw) (`KismetMathLibrary.BreakRotator` (`KismetMathLibrary.Quat_Rotator` Q1)))
  (bind (_returnvalue_roll_2 _returnvalue_pitch_2 _returnvalue_yaw_2) (`KismetMathLibrary.BreakRotator` (`KismetMathLibrary.Quat_Rotator` parent)))
  (return (`KismetMathLibrary.InverseTransformRotation` (`KismetMathLibrary.MakeTransform` `T Location` (`KismetMathLibrary.MakeRotator` _returnvalue_roll_2 (* -1 _returnvalue_pitch_2) (* -1 _returnvalue_yaw_2))) (`KismetMathLibrary.MakeRotator` _returnvalue_roll (* -1 _returnvalue_pitch) (* -1 _returnvalue_yaw)))))

(fn `UserConstructionScript`)