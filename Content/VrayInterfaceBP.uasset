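; Bridge actor between Unreal and a V-Ray scene, creating render view and physical camera plugins with matching actors on BeginPlay.
; Wraps C++ calls to load scenes, read and write plugin parameters, and delete selected plugins with their actors.
; Manages click selection with Shift-add, Alt ignore and highlight feedback.
; The routine for spawning actors from loaded plugins has its spawn branches disconnected.
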(event `self.ReceiveBeginPlay`
  (bind _pluginnameout (`self.CreatePluginCpp` "ERenderView"))
  (`|SpawnActorFromClass` "/Game/RndrBaseActor_renderView.RndrBaseActor_renderView_C" (`KismetMathLibrary.MakeTransform` (0.0 0.0 0.0)) "Undefined" "OverrideRootScale" null _pluginnameout null)
  (bind _pluginnameout_2 (`self.CreatePluginCpp` "EPhysicalCamera"))
  (`|SpawnActorFromClass` "/Game/RndrBaseActor_PhysCamera.RndrBaseActor_PhysCamera_C" (`KismetMathLibrary.MakeTransform` (0.0 0.0 0.0)) "Undefined" "OverrideRootScale" null _pluginnameout_2 null))

(fn `Delete`
  (locals (Obj :type "/Game/RndrBaseActor Object Reference"))
  (for _array_element (`self.GetSelection`)
    (set `local.Obj` _array_element)
    (bind _returnvalue (`self.DeletePluginCpp` (`/Game/RndrBaseActor.name` (`local.Obj`))))
    (if _returnvalue
      (`self.K2_DestroyActor` (`local.Obj`))))
  (return))

(fn `GetInfoABC`
  (params (PluginType :type "EVrayPluginType Enum" :default "ENode") (nameIn :type String) (ParameterName :type String))
  (returns (l_propertyName1 :type "Array of String") (l_propertyValue1 :type "Array of String") (l_propertyType1 :type "Array of String"))
  (locals (transformOut :type "Array of Vector Structure") (l_propertyName :type "Array of String") (l_propertyValue :type "Array of String") (l_PropertyType :type "Array of String"))
  (bind (_propertynamesout _propertyvaluesout _paramtypeout) (`self.GetVrayPluginParameter` PluginType nameIn ParameterName))
  (set `local.l_propertyName` _propertynamesout)
  (set `local.l_propertyValue` _propertyvaluesout)
  (set `local.l_PropertyType` _paramtypeout)
  (return (`local.l_propertyName`) (`local.l_propertyValue`) (`local.l_PropertyType`)))

(fn `GetSelection`
  (returns (Selection :type "Array of /Game/RndrBaseActor Object Reference") (PluginType1 :type "EVrayPluginType Enum"))
  (locals (PluginType :type "EVrayPluginType Enum"))
  (`|ExecutionSequence`
    (:`then_0`
      (switch `string` (`KismetSystemLibrary.GetClassDisplayName` (`GameplayStatics.GetObjectClass` (`|GetArrayItem` (`self.Selection`))))
        (:`RndrBaseActor_Node_C`
          (set `local.PluginType` "EBRDF"))
        (:`RndrBaseActor_Light_C`
          (set `local.PluginType` "ELightSphere"))
        (:`RndrBaseActor_renderView_C`
          (set `local.PluginType` "ERenderView"))))
    (:`then_1`
      (return (`self.Selection`) (`local.PluginType`)))))

(fn `GetVraySceneInfo`
  (params (path :type String))
  (returns (typeOut :type "Array of String") (nameOut :type "Array of String"))
  (bind (_plugintype _pluginname) (`self.GetVrayNodeNames`))
  (`self.LoadScene` path)
  (return _plugintype _pluginname))

(fn `readVrayPluginsAndSpawnUnrealEquivalent`
  (locals (index :type Integer) (name :type "Array of String") (type :type "Array of String") (lightType :type Integer :default 0) (PluginName :type String))
  (bind (_plugintype _pluginname) (`self.GetVrayNodeNames`))
  (set `local.type` _plugintype)
  (set `local.name` _pluginname)
  (for (_array_element _array_index) (`local.type`)
    (set `local.index` _array_index)
    (set `local.PluginName` (`|GetArrayItem` (`local.name`) (`local.index`)))
    (switch `string` _array_element)))

(fn `SetInfoABC`
  (params (ParameterName :type String) (PluginType :type "EVrayPluginType Enum" :default "ENode") (nameIn :type String) (transformIn :type "Array of Vector Structure") (colorIn :type "LinearColor Structure") (intIn :type Integer) (floatArrayIn :type "Array of Float (double-precision)"))
  (returns (ParamSetSuccessfully :type Boolean))
  (locals (ParamName :type String) (FloatArray :type "Array of Float (double-precision)") (Transform :type "Array of Vector Structure") (bReinicializarRender :type Boolean :default false))
  (set `local.bReinicializarRender` (select `EVrayPluginType` PluginType :`EPhysicalCamera` true))
  (set `local.ParamName` ParameterName)
  (set `local.FloatArray` floatArrayIn)
  (set `local.Transform` transformIn)
  (bind _paramsetsuccessfully (`self.SetVrayPluginParameter` PluginType (`local.Transform`) nameIn colorIn intIn (`local.FloatArray`) (`local.ParamName`) (`local.bReinicializarRender`)))
  (return _paramsetsuccessfully))

(fn `SetSelectionRndrd`
  (params (baseActorIn :type "/Game/RndrBaseActor Object Reference"))
  (locals (BaseActor :type "/Game/RndrBaseActor Object Reference"))
  (set `local.BaseActor` baseActorIn)
  (if (not (`PlayerController.IsInputKeyDown` (`GameplayStatics.GetPlayerController` 0) "LeftAlt"))
    (if (not (`PlayerController.IsInputKeyDown` (`GameplayStatics.GetPlayerController` 0) "LeftShift"))
      (for _array_element (`self.Selection`)
        (`/Game/RndrBaseActor.EnableSelectionFeedback` _array_element false))
      (`KismetArrayLibrary.Array_Clear` (`self.Selection`)))
    (`KismetArrayLibrary.Array_AddUnique` (`self.Selection`) (`local.BaseActor`))
    (for _array_element_2 (`self.Selection`)
      (`/Game/RndrBaseActor.EnableSelectionFeedback` _array_element_2 true))
    (return)
    (else
      (return))))

(fn `UserConstructionScript`)