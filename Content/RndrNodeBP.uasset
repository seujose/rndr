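; RndrNodeBP is an actor that visualizes a V-Ray scene node in the world as a colored box.
; After a short delay on BeginPlay, it builds a procedural box mesh with collision and a dynamic instance of the master material.
; Using the game instance's V-Ray interface, it looks up plugin parameters by name, placing itself from the node transform and tinting BaseColor from the BRDF diffuse color.
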(event `self.ReceiveBeginPlay`
  (set `self.VrayInst` (`/Game/RndrGameInstanceBP.VrayInterface` (cast `/Game/RndrGameInstanceBP` (`GameplayStatics.GetGameInstance`) :!pure true)))
  (`KismetSystemLibrary.Delay` 0.2)
  (`self.CreateNode`))

(event `self.BP_OnItemSelectionChanged`
  (params (bIsSelected :type Boolean))
  (if bIsSelected
    _))

(fn `CreateNode`
  (bind (_vertices _triangles _normals _uvs _tangents) (`KismetProceduralMeshLibrary.GenerateBoxMesh` (25.0 25.0 25.0)))
  (`ProceduralMeshComponent.CreateMeshSection_LinearColor` :`self` (`self.ProceduralMesh`) :`Vertices` _vertices :`Triangles` _triangles :`Normals` _normals :`UV0` _uvs :`Tangents` _tangents :`bCreateCollision` true)
  (bind _returnvalue (`PrimitiveComponent.CreateDynamicMaterialInstance` (`self.ProceduralMesh`) 0 "/Game/MasterMaterial.MasterMaterial" "None"))
  (set `self.Mat` _returnvalue)
  (bind _transformout (`VrayInterface.GetVrayPluginParameter` (`self.VrayInst`) "ENode" (`self.name`) "transform"))
  (`self.K2_SetActorLocation` (`|GetArrayItem` _transformout 3) false true)
  (bind (_transformout_2 _colorout) (`VrayInterface.GetVrayPluginParameter` (`self.VrayInst`) "EBRDF" (`self.name`) "diffuse"))
  (`MaterialInstanceDynamic.SetVectorParameterValue` (`self.Mat`) "BaseColor" _colorout)
  (return))

(fn `GetListItemObject`
  (returns (ReturnValue :type "Object Object Reference"))
  (return null))

(fn `UserConstructionScript`)