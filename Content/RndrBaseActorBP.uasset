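; RndrBaseActorBP is a base actor that shows a text label turned toward the player.
; Each tick, TextLookAt copies the TextTextComponent value into TextRender and rotates it along the look-at direction from the actor's location to player character 0.
; BeginPlay, the construction script and the list-item functions (OnItemSelectionChanged, GetListItemObject) are empty stubs.
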(event `self.ReceiveBeginPlay`)

(event `self.ReceiveTick`
  (params (DeltaSeconds :type "Float (single-precision)"))
  (`self.TextLookAt`))

(event `self.BP_OnItemSelectionChanged`
  (params (bIsSelected :type Boolean))
  (if bIsSelected
    _))

(fn `GetListItemObject`
  (returns (ReturnValue :type "Object Object Reference"))
  (return null))

(fn `TextLookAt`
  (`TextRenderComponent.K2_SetText` (`self.TextRender`) (`self.textTextComponent`))
  (`SceneComponent.K2_SetWorldRotation` (`self.TextRender`) (`KismetMathLibrary.FindLookAtRotation` (`self.K2_GetActorLocation`) (`self.K2_GetActorLocation` (`GameplayStatics.GetPlayerCharacter` 0))) false true))

(fn `UserConstructionScript`)